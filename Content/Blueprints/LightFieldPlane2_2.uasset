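; Prototype light field plane actor that sets up a dynamic material on its ImagePlane and draws debug points from that plane's bounds.
; The construction script creates and stores the material instance, and BeginPlay pushes a fixed vector into TestParam.
; Tick runs a 16x16 loop, but every iteration draws at the same rotated-extent offset from the bounds origin.
; Per-cell grid math and a camera location print are left unconnected.
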(event `self.ReceiveBeginPlay`
  (`MeshComponent.SetVectorParameterValueOnMaterials` (`self.ImagePlane`) "TestParam" (`KismetMathLibrary.MakeVector` 0.0 100.0 100.0)))

(event `self.ReceiveTick`
  (params (DeltaSeconds :type "Float (single-precision)"))
  (bind (_origin _boxextent) (`KismetSystemLibrary.GetComponentBounds` (`self.ImagePlane`)))
  (for _index (range 16)
    (for _index_2 (range 16)
      (`KismetSystemLibrary.DrawDebugPoint` (+ _origin (`KismetMathLibrary.GreaterGreater_VectorRotator` _boxextent (`SceneComponent.K2_GetComponentRotation` (`self.ImagePlane`)))) 50.0 (struct :`R` 1.0 :`G` 0.25428 :`B` 0.862845 :`A` 1.0) 10.0))))

(fn `UserConstructionScript`
  (bind _returnvalue (`PrimitiveComponent.CreateDynamicMaterialInstance` (`self.ImagePlane`) 0 null))
  (set `self.Material` _returnvalue))
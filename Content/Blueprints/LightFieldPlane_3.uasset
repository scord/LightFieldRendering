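; Actor that displays a light field on an image plane using an auto-focus material.
; The construction script creates a dynamic material instance and feeds it aperture, sensor, resolution, focus and depth parameters.
; Focal length scales with the plane's world scale, the focus vectors follow its up vector, and depth scale derives from plane size, grid size and Dist.
; The event graph is empty, and LightFieldTexture is unused.
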(event `self.ReceiveBeginPlay`)

(fn `UserConstructionScript`
  (bind _imageplane (`self.ImagePlane`))
  (bind _imageplane_2 (`self.ImagePlane`))
  (bind _focus_distance (`self.Focus Distance`))
  (bind _imageplane_3 (`self.ImagePlane`))
  (bind _imagescale (`self.ImageScale`))
  (bind _resolution (`self.Resolution`))
  (bind (_x _y) (`KismetMathLibrary.BreakVector2D` _resolution))
  (bind _returnvalue (`SceneComponent.GetUpVector` (`self.ImagePlane`)))
  (bind _x_2 (.x (`SceneComponent.K2_GetComponentScale` _imageplane_2)))
  (bind _returnvalue_2 (* _x_2 (`self.Focal Length`)))
  (bind _returnvalue_3 (/ (/ (* _x_2 100.0) (`KismetMathLibrary.Conv_IntToDouble` (`self.Grid Size`))) (`self.Dist`)))
  (bind _returnvalue_4 (`PrimitiveComponent.CreateDynamicMaterialInstance` _imageplane_2 0 "/Game/Blueprints/LightFieldMaterial_AutoFocus.LightFieldMaterial_AutoFocus"))
  (set `self.Material` _returnvalue_4)
  (`MeshComponent.SetScalarParameterValueOnMaterials` _imageplane_2 "ApertureSize" (/ 1000.0 (`self.ApertureSize`)))
  (`MeshComponent.SetVectorParameterValueOnMaterials` _imageplane_2 "SensorSize" (`KismetMathLibrary.MakeVector` _imagescale (* _imagescale (/ _y _x))))
  (`MeshComponent.SetVectorParameterValueOnMaterials` (`self.ImagePlane`) "Resolution" (`KismetMathLibrary.Conv_Vector2DToVector` _resolution))
  (`MeshComponent.SetVectorParameterValueOnMaterials` (`self.ImagePlane`) "FocusVector" (* _returnvalue _returnvalue_2))
  (`MeshComponent.SetVectorParameterValueOnMaterials` (`self.ImagePlane`) "FocusVector2" _returnvalue)
  (`MeshComponent.SetScalarParameterValueOnMaterials` _imageplane "FocusRatio" (/ _returnvalue_2 (* _returnvalue_3 _focus_distance)))
  (`MeshComponent.SetScalarParameterValueOnMaterials` _imageplane "FocalLength" _returnvalue_2)
  (`MeshComponent.SetScalarParameterValueOnMaterials` (`self.ImagePlane`) "DepthScale" _returnvalue_3)
  (`MeshComponent.SetScalarParameterValueOnMaterials` _imageplane_3 "FocusDistance" _focus_distance)
  (`MeshComponent.SetScalarParameterValueOnMaterials` _imageplane_3 "DepthThreshold" (`self.DepthThreshold`))
  (`MeshComponent.SetScalarParameterValueOnMaterials` _imageplane_3 "FocusIterations" (`KismetMathLibrary.Conv_IntToDouble` (`self.FocusIterations`))))
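; LightFieldPlane is an actor that configures an image plane's material, apparently for light field rendering with adjustable aperture and focus.
; Its construction script creates a dynamic material instance on ImagePlane, then pushes aperture, sensor size, resolution and two focus vectors as parameters.
; Sensor size follows world X scale, ImageScale and resolution aspect, while focus vectors follow the plane's up vector scaled by focal length or focus distance.
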(event `self.ReceiveBeginPlay`)

(fn `UserConstructionScript`
  (bind _imageplane (`self.ImagePlane`))
  (bind _resolution (`self.Resolution`))
  (bind _returnvalue (`SceneComponent.K2_GetComponentScale` _imageplane))
  (bind (_x _y) (`KismetMathLibrary.BreakVector2D` _resolution))
  (bind _returnvalue_2 (`SceneComponent.GetUpVector` (`self.ImagePlane`)))
  (bind _returnvalue_3 (* (.x _returnvalue) (`self.ImageScale`)))
  (bind _returnvalue_4 (`PrimitiveComponent.CreateDynamicMaterialInstance` _imageplane 0 null))
  (set `self.Material` _returnvalue_4)
  (`MeshComponent.SetScalarParameterValueOnMaterials` _imageplane "ApertureSize" (/ 1000.0 (`self.ApertureSize`)))
  (`MeshComponent.SetVectorParameterValueOnMaterials` _imageplane "SensorSize" (`KismetMathLibrary.MakeVector` _returnvalue_3 (* _returnvalue_3 (/ _y _x))))
  (`MeshComponent.SetVectorParameterValueOnMaterials` (`self.ImagePlane`) "Resolution" (`KismetMathLibrary.Conv_Vector2DToVector` _resolution))
  (`MeshComponent.SetVectorParameterValueOnMaterials` (`self.ImagePlane`) "FocusVector" (* (* _returnvalue (`self.Focal Length`)) _returnvalue_2))
  (`MeshComponent.SetVectorParameterValueOnMaterials` (`self.ImagePlane`) "FocusVector2" (* _returnvalue_2 (`self.Focus Distance`))))